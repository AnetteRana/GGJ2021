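; BP_Poster is a poster actor that features one of five special cats and spawns that cat into the level.
; On BeginPlay it rolls a random CatID, applies the matching cat material to the Poster component, and spawns the matching BP_Cat class at a random SpecialCatSpawnPoint, stamped with that ID.
; MakeNewPoster clears the material, waits a few seconds, then loops back into the same roll-and-spawn logic.
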(event `self.ReceiveBeginPlay`
  ;[1 1 1] set random ID
  (bind _output_get (set `self.CatID` (`KismetMathLibrary.RandomIntegerInRange` 1 5) :!label _label))
  (bind _outactors (`GameplayStatics.GetAllActorsOfClass` "/Game/myCatPlacement/SpecialCatSpawnPoint.SpecialCatSpawnPoint_C"))
  ;[1 1 1] Set material
  (switch `int` _output_get
    (:`1`
      (`PrimitiveComponent.SetMaterial` (`self.Poster`) 0 "/Game/CatsAndPosters/Materials/Cat_B_W_Stripes.Cat_B_W_Stripes")
      (bind _returnvalue (`KismetMathLibrary.MakeTransform` (`SceneComponent.K2_GetComponentLocation` (`/Game/myCatPlacement/SpecialCatSpawnPoint.DefaultSceneRoot` (`KismetArrayLibrary.Array_Random` _outactors)))))
      (bind _returnvalue_2 (`|SpawnActorFromClass` "/Game/CatsAndPosters/BP_Cat_A.BP_Cat_A_C" _returnvalue "Undefined" "OverrideRootScale" null null))
      (set `/Game/BP_Cat.catID` 1 _returnvalue_2))
    (:`2`
      (`PrimitiveComponent.SetMaterial` (`self.Poster`) 0 "/Game/CatsAndPosters/Materials/Cat_Leo.Cat_Leo")
      (bind _returnvalue_3 (`|SpawnActorFromClass` "/Game/CatsAndPosters/BP_Cat_B.BP_Cat_B_C" _returnvalue "Undefined" "OverrideRootScale" null null))
      (set `/Game/BP_Cat.catID` 2 _returnvalue_3))
    (:`3`
      (`PrimitiveComponent.SetMaterial` (`self.Poster`) 0 "/Game/CatsAndPosters/Materials/Cat_Black.Cat_Black")
      (bind _returnvalue_4 (`|SpawnActorFromClass` "/Game/CatsAndPosters/BP_Cat_C.BP_Cat_C_C" _returnvalue "Undefined" "OverrideRootScale" null null))
      (set `/Game/BP_Cat.catID` 3 _returnvalue_4))
    (:`4`
      (`PrimitiveComponent.SetMaterial` (`self.Poster`) 0 "/Game/CatsAndPosters/Materials/Cat_O_B.Cat_O_B")
      (bind _returnvalue_5 (`|SpawnActorFromClass` "/Game/CatsAndPosters/BP_Cat_D.BP_Cat_D_C" _returnvalue "Undefined" "OverrideRootScale" null null))
      (set `/Game/BP_Cat.catID` 4 _returnvalue_5))
    (:`5`
      (`PrimitiveComponent.SetMaterial` (`self.Poster`) 0 "/Game/CatsAndPosters/Materials/Cat_Orange.Cat_Orange")
      (bind _returnvalue_6 (`|SpawnActorFromClass` "/Game/CatsAndPosters/BP_Cat_E.BP_Cat_E_C" _returnvalue "Undefined" "OverrideRootScale" null null))
      (set `/Game/BP_Cat.catID` 5 _returnvalue_6))))

(event `Make New Poster`
  (`PrimitiveComponent.SetMaterial` (`self.Poster`) 0 null)
  (`KismetSystemLibrary.Delay` 7.0)
  (goto _label))

(fn `UserConstructionScript`)