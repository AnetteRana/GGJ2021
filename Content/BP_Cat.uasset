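; BP_Cat is a wandering cat actor that roams around the spot where it begins play.
; Each tick, unless IsPickedUp is set, it steps forward and curves left or right by a random yaw amount.
; A random countdown periodically re-rolls the turn direction, and straying too far snaps its facing back toward home.
; Movement and turning are per frame, not scaled by delta time.
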(event `setHome`
  ;[1 1 1] set home
  (set `self.homeLoc` (`SceneComponent.K2_GetComponentLocation` (`self.BW_Cat`)) :!label _label)
  (`self.set turn direction`))

(event `self.ReceiveBeginPlay`
  (goto _label))

(event `directionChanger`
  (params (NewParam :type "Float (double-precision)"))
  ;[1 1 1] direction changer
  (bind _output_get (set `self.turnCountdown` (- (stale _output_get) NewParam)))
  (if (<= (`self.turnCountdown`) 0.0)
    (set `self.turnCountdown` (`KismetMathLibrary.RandomFloatInRange` 3.0 6.0))
    (`self.set turn direction`)))

(event `self.ReceiveTick`
  (params (DeltaSeconds :type "Float (single-precision)"))
  (bind _defaultsceneroot (`self.DefaultSceneRoot`))
  (`self.directionChanger` DeltaSeconds)
  ;[1 1 1] not held?
  (if (not (`self.IsPickedUp`))
    ;[1 1 1] straying far?
    (if (> (`KismetMathLibrary.VSize` (- (`SceneComponent.K2_GetComponentLocation` (`self.DefaultSceneRoot`)) (`self.homeLoc`))) 200.0)
      ;[1 1 1] turn back
      (`self.K2_SetActorRotation` (`KismetMathLibrary.Conv_VectorToRotator` (- (`self.homeLoc`) (`SceneComponent.K2_GetComponentLocation` (`self.BW_Cat`))))))
    ;[1 1 1] walk randomly
    (`SceneComponent.K2_SetWorldLocationAndRotation` _defaultsceneroot (+ (`SceneComponent.K2_GetComponentLocation` _defaultsceneroot) (* (`SceneComponent.GetForwardVector` _defaultsceneroot) (`self.walkSpeed`))) (`KismetMathLibrary.MakeRotator` (.roll (`SceneComponent.K2_GetComponentRotation` _defaultsceneroot)) (.pitch (`SceneComponent.K2_GetComponentRotation` _defaultsceneroot)) (+ (.yaw (`SceneComponent.K2_GetComponentRotation` _defaultsceneroot)) (* (`KismetMathLibrary.RandomFloatInRange` 0.3 0.6) (`KismetMathLibrary.Conv_IntToDouble` (`self.turnDirection`))))) false false)))

(event `set turn direction`
  ;[1 1 1] set random direction to turn
  (switch `int` (`KismetMathLibrary.RandomIntegerInRange` 0 1)
    (:`Default`
      (set `self.turnDirection` -1))
    (:`0`
      (set `self.turnDirection` 1))))

(fn `UserConstructionScript`)